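; BP_Button is a button actor that counts how many times a VRPawn begins overlapping its Box component.
; Each such overlap increments TotalPumps and prints the new total as debug text.
; BeginPlay caches the Button component's relative location in ButtonStart, but the button never moves, as the node computing a lowered position is left unconnected.
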(event OnComponentBeginOverlap(Box)
  (params (OverlappedComponent :type Primitive%20Component%20Object%20Reference) (OtherActor :type Actor%20Object%20Reference) (OtherComp :type Primitive%20Component%20Object%20Reference) (OtherBodyIndex :type Integer) (bFromSweep :type Boolean) (SweepResult :type Hit%20Result%20Structure%20%28by%20ref%29))
  (Utilities|Casting|CastToVRPawn OtherActor)
  (Variables|Default|SetTotalPumps (+ (Variables|Default|GetTotalPumps) 1))
  (Development|PrintString (Utilities|String|ToString(Integer) (Variables|Default|GetTotalPumps))))

(event EventBeginPlay
  (Variables|Default|SetButtonStart (Variables|/Script/Engine.SceneComponent|GetRelativeLocation (Variables|Default|GetButton))))

(event Collision|EventActorBeginOverlap
  (params (OtherActor :type Actor%20Object%20Reference)))

(fn ConstructionScript)